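; AI controller for an enemy AiCharacter that runs a behavior tree on possession and keeps a reference to the pawn.
; Perception updates for the player character set CanSeePlayer on the blackboard; losing the player stores their current position as PlayerLocation and clears the flag.
; Walk, Run and Attack events forward to the possessed enemy, while a RecentlySighted blackboard write is left unconnected.
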(event `self.AIPerception.OnTargetPerceptionUpdated`
  (params (Actor :type "Actor Object Reference") (Stimulus :type "AIStimulus Structure"))
  (bind (_age _expirationage _strength _stimuluslocation _receiverlocation _tag _bsuccessfullysensed) (break `AIStimulus` Stimulus))
  (bind _returnvalue (`AIBlueprintHelperLibrary.GetBlackboard` null))
  ;[1 1 1] Allows variable value to change if enemy see's character
  (cast `/Game/ThirdPersonBP/Blueprints/ThirdPersonCharacter` Actor)
  (`BlackboardComponent.SetValueAsBool` _returnvalue "CanSeePlayer" _bsuccessfullysensed)
  (if (not _bsuccessfullysensed)
    (`BlackboardComponent.SetValueAsVector` _returnvalue "PlayerLocation" (`self.K2_GetActorLocation` (`GameplayStatics.GetPlayerCharacter` 0)))
    (`BlackboardComponent.ClearValue` _returnvalue "CanSeePlayer")))

(event `Walk`
  ;[1 1 1] Events referenced to object type
  (`/Game/AI/AiCharacter.Walk` (`self.enemy`)))

(event `Run`
  ;[1 1 1] Events referenced to object type
  (`/Game/AI/AiCharacter.Run` (`self.enemy`)))

(event `self.OnPossess`
  (params (PossessedPawn :type "Pawn Object Reference"))
  ;[1 1 1] Behavior tree is ran to ai character
  (bind _asai_character (cast `/Game/AI/AiCharacter` PossessedPawn))
  (set `self.enemy` _asai_character)
  (`self.RunBehaviorTree` "/Game/AI/Tree.Tree"))

(event `Attack`
  ;[1 1 1] Allows ai to attack
  (`/Game/AI/AiCharacter.Attack` (`self.enemy`)))

(fn `UserConstructionScript`)