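; Sword-wielding enemy AI character that can walk, run and slash at the player.
; Attack plays a one-shot slash animation and sound and holds an Attacking flag for a timed window, during which capsule overlaps damage ThirdPersonCharacter.
; The construction script attaches the weapon mesh to the WeaponSocket.
; It also carries pause, unpause and death-screen widget functions, none called within this Blueprint.
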(event `self.Capsule.OnComponentBeginOverlap`
  (params (OverlappedComponent :type "PrimitiveComponent Object Reference") (OtherActor :type "Actor Object Reference") (OtherComp :type "PrimitiveComponent Object Reference") (OtherBodyIndex :type Integer) (bFromSweep :type Boolean) (SweepResult :type "HitResult Structure (by ref)"))
  ;[1 1 1] Character takes damage from sword
  (if (`self.Attacking`)
    (bind _asthird_person_character (cast `/Game/ThirdPersonBP/Blueprints/ThirdPersonCharacter` OtherActor))
    (`/Game/ThirdPersonBP/Blueprints/ThirdPersonCharacter.TakeDamage` _asthird_person_character 10)))

(event `Walk`
  ;[1 1 1] Sets AI Speed
  (set `CharacterMovementComponent.MaxWalkSpeed` 150.0 (`self.CharacterMovement`)))

(event `Run`
  ;[1 1 1] Sets AI Speed
  (set `CharacterMovementComponent.MaxWalkSpeed` 400.0 (`self.CharacterMovement`)))

(event `Attack`
  ;[1 1 1] AI attack animation and sound
  (`SkeletalMeshComponent.PlayAnimation` (`self.Mesh`) "/Game/MixamoAnimPack/Mixamo_Mortimer/Anims/Mortimer_Sword_Slash.Mortimer_Sword_Slash" false)
  (`GameplayStatics.SpawnSoundAttached` "/Game/AI/EnemySwordCue.EnemySwordCue" (`self.StaticMesh`))
  (set `self.Attacking` true)
  (`KismetSystemLibrary.Delay` 1.5)
  (set `self.Attacking` false)
  (`SkeletalMeshComponent.SetAnimationMode` (`self.Mesh`) "AnimationBlueprint"))

(fn `DeathMsg`
  (`Widget.SetVisibility` (`self.YouDied`) "Visible")
  (`/Engine/EditorBlueprintResources/StandardMacros.IsValid` (`self.YouDied`)
    (:`Is Valid`
      _)
    (:`Is Not Valid`
      (bind _returnvalue (`|CreateWidget` "/Game/Menus/YouDied.YouDied_C" (`GameplayStatics.GetPlayerController` 0)))
      (set `self.YouDied` _returnvalue)))
  (`UserWidget.AddToViewport` (`self.YouDied`) 0)
  (`WidgetBlueprintLibrary.SetInputMode_UIOnlyEx` (`GameplayStatics.GetPlayerController` 0) (`self.YouDied`))
  (set `PlayerController.bShowMouseCursor` true (`GameplayStatics.GetPlayerController` 0)))

(fn `PauseGame`
  (`Widget.SetVisibility` (`self.Pause Menu`) "Visible")
  (`GameplayStatics.SetGamePaused` true)
  (`/Engine/EditorBlueprintResources/StandardMacros.IsValid` (`self.Pause Menu`)
    (:`Is Valid`
      _)
    (:`Is Not Valid`
      (bind _returnvalue (`|CreateWidget` "/Game/Menus/PauseMenuWidget1.PauseMenuWidget1_C" (`GameplayStatics.GetPlayerController` 0)))
      (set `self.Pause Menu` _returnvalue)))
  (`UserWidget.AddToViewport` (`self.Pause Menu`) 0)
  (`WidgetBlueprintLibrary.SetInputMode_UIOnlyEx` (`GameplayStatics.GetPlayerController` 0) (`self.Pause Menu`))
  (set `PlayerController.bShowMouseCursor` true (`GameplayStatics.GetPlayerController` 0)))

(fn `UnpauseGame`
  (bind _returnvalue (`GameplayStatics.GetPlayerController` 0))
  (`GameplayStatics.SetGamePaused` false)
  (`Widget.SetVisibility` (`self.Pause Menu`) "Hidden")
  (`WidgetBlueprintLibrary.SetInputMode_GameOnly` _returnvalue)
  (set `PlayerController.bShowMouseCursor` false _returnvalue))

(fn `UserConstructionScript`
  (`SceneComponent.K2_AttachToComponent` (`self.StaticMesh`) (`self.Mesh`) "WeaponSocket" "KeepRelative" "KeepRelative" "KeepRelative" true))